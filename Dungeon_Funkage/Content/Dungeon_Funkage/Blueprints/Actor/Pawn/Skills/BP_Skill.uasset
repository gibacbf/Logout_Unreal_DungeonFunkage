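; BP_Skill is a skill actor that stores its caster, description, attributes and costs through setter events.
; ExecuteSkill deducts health, mana and stamina costs from the given character, then activates projectile movement for Bullet-behavior skills.
; Overlaps on the effect range collision apply the skill's damage to BP_Character_Enemy actors only.
; Cooldown, level and caster are stored but not used in this graph.
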(event OnComponentBeginOverlap(Effect_Range_Collision)
  (params (OverlappedComponent :type Primitive%20Component%20Object%20Reference) (OtherActor :type Actor%20Object%20Reference) (OtherComp :type Primitive%20Component%20Object%20Reference) (OtherBodyIndex :type Integer) (bFromSweep :type Boolean) (SweepResult :type Hit%20Result%20Structure%20%28by%20ref%29))
  (CallFunction|DamageObject OtherActor))

(event Custom|WhoCasted
  (params (Caster :type BP%20Character%20Funkage%20Object%20Reference))
  (Variables|Default|SetCaster Caster))

(event Custom|ExecuteSkill
  (params (Character :type BP%20Character%20Funkage%20Object%20Reference))
  (CallFunction|SkillReduceHealth Character)
  (CallFunction|SkillReduceMana Character)
  (CallFunction|SkillReduceStamina Character)
  (switch Utilities|FlowControl|Switch|SwitchonEnum_SkillType_Behavior (Variables|SkillDesc|GetSkillBehavior)
    (:NewEnumerator0
      (Components|Activation|SetActive (Variables|Default|GetProjectileMovement) true false))))

(event Custom|SkillReduceMana
  (params (Character :type BP%20Character%20Funkage%20Object%20Reference))
  ;[0.04166 0.998 1] Character Functions
  (Default|CharacterReduceMana Character (Variables|SkillCost|GetManaCost)))

(event Custom|SkillReduceStamina
  (params (Character :type BP%20Character%20Funkage%20Object%20Reference))
  ;[0.04166 0.998 1] Character Functions
  (Default|CharacterReduceStamina Character (Variables|SkillCost|GetStaminaCost)))

(event Custom|SkillReduceHealth
  (params (Character :type BP%20Character%20Funkage%20Object%20Reference))
  ;[0.04166 0.998 1] Character Functions
  (Default|CharacterReduceLife Character (Variables|SkillCost|GetHealthCost)))

(event Custom|DamageObject
  (params (Object :type Object%20Object%20Reference))
  ;[0.04166 0.998 1] Character Functions
  (bind _asbp_character_enemy (Utilities|Casting|CastToBP_Character_Enemy Object))
  (Default|CharacterReduceLife _asbp_character_enemy (Variables|SkillStributes|GetDamagePoints)))

(event Custom|SetSkillAttributes
  (params (Damage :type Integer) (CoolDown :type Float%20%28single-precision%29))
  (Variables|SkillStributes|SetDamagePoints Damage)
  (Variables|SkillStributes|SetCooldown CoolDown))

(event Custom|SetSkillCost
  (params (ManaCost :type Integer) (StaminaCost :type Integer) (HealthCost :type Integer))
  (Variables|SkillCost|SetManaCost ManaCost)
  (Variables|SkillCost|SetStaminaCost StaminaCost)
  (Variables|SkillCost|SetHealthCost HealthCost))

(event Custom|SetSkillDesc
  (params (Name :type String) (SkillBehavior :type Enum_SkillType_Behavior%20Enum :default "NewEnumerator0") (SkillLevel :type Enum_SkillType_Level%20Enum :default "NewEnumerator0"))
  (Variables|SkillDesc|SetName Name)
  (Variables|SkillDesc|SetSkillBehavior SkillBehavior)
  (Variables|SkillDesc|SetSkillLevel SkillLevel))

(fn ConstructionScript)