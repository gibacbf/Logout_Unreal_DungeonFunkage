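; BP_Character_Funkage is a character Blueprint for Dungeon Funkage that holds health, mana, stamina and damage attributes, with events to set or reduce them.
; An AttackRange overlap component keeps a RangedEnemies list of other Funkage characters, with no team filter.
; CharacterAttack applies damage to everyone on that list.
; CharacterDeathCondition destroys the actor at zero health but is not called within this graph, and CharacterUseSkill is an empty stub.
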(event OnComponentBeginOverlap(AttackRange)
  (params (OverlappedComponent :type Primitive%20Component%20Object%20Reference) (OtherActor :type Actor%20Object%20Reference) (OtherComp :type Primitive%20Component%20Object%20Reference) (OtherBodyIndex :type Integer) (bFromSweep :type Boolean) (SweepResult :type Hit%20Result%20Structure%20%28by%20ref%29))
  (bind _asbp_character_funkage (Utilities|Casting|CastToBP_Character_Funkage OtherActor))
  (Utilities|Array|Add (Variables|Default|GetRangedEnemies) _asbp_character_funkage))

(event OnComponentEndOverlap(AttackRange)
  (params (OverlappedComponent :type Primitive%20Component%20Object%20Reference) (OtherActor :type Actor%20Object%20Reference) (OtherComp :type Primitive%20Component%20Object%20Reference) (OtherBodyIndex :type Integer))
  (bind _asbp_character_funkage (Utilities|Casting|CastToBP_Character_Funkage OtherActor))
  (Utilities|Array|RemoveItem (Variables|Default|GetRangedEnemies) _asbp_character_funkage))

(event Custom|CharacterAttack
  (params (Damage :type Integer))
  ;[1 0.8447 0] Character Combat
  (for _array_element (Variables|Default|GetRangedEnemies)
    (CallFunction|CharacterReduceLife _array_element Damage)))

(event Custom|CharacterUseSkill
  ;[1 0.8447 0] Character Combat
)

(event Custom|CharacterReduceStamina
  (params (StaminaCost :type Integer))
  ;[1 0 0.08048] Character Attributes
  (Variables|BasicAtributes|SetStaminaPoints (- (Variables|BasicAtributes|GetStaminaPoints) StaminaCost)))

(event Custom|CharacterReduceMana
  (params (ManaCost :type Integer))
  ;[1 0 0.08048] Character Attributes
  (Variables|BasicAtributes|SetManaPoints (- (Variables|BasicAtributes|GetManaPoints) ManaCost)))

(event Custom|CharacterReduceLife
  (params (Damage :type Integer))
  ;[1 0 0.08048] Character Attributes
  (Variables|BasicAtributes|SetHealthPoints (- (Variables|BasicAtributes|GetHealthPoints) Damage)))

(event Custom|CharacterDeathCondition
  ;[1 0.8447 0] Character Combat
  (if (<= (Variables|BasicAtributes|GetHealthPoints) 0)
    (Actor|DestroyActor)))

(event Custom|SetBasicAttributes
  (params (Health :type Integer) (Mana :type Integer) (Stamina :type Integer))
  (Variables|BasicAtributes|SetHealthPoints Health)
  (Variables|BasicAtributes|SetManaPoints Mana)
  (Variables|BasicAtributes|SetStaminaPoints Stamina))

(event Custom|SetCombatAttributes
  (params (Damage :type Integer))
  (Variables|CombatAttributes|SetDamagePoints Damage))

(fn ConstructionScript)