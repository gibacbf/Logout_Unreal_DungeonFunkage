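; Player character Blueprint that handles movement, melee attacks and skill casting, and checks its death condition every tick.
; BeginPlay sets health, mana, stamina and damage attributes.
; Movement is turn-and-advance: the forward axis moves along control yaw, while the right axis rotates the controller instead of strafing.
; Skills spawn by tier from a class array at the ranged skill position, though only melee and basic skill have input bindings.
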(event Custom|PlayerAttack
  ;[1 0.02399 0] Combat
  ;;[1 0.904 0] CharacterStuff
  (CallFunction|CharacterAttack (Variables|Default|GetDamagePoints)))

(event Custom|PlayerExecuteSkill
  (params (SkillLevel :type Enum_SkillType_Level%20Enum :default "NewEnumerator0"))
  ;[1 0.02399 0] Combat
  ;;[0 1 0.1595] SkillStuff
  (switch Utilities|FlowControl|Switch|SwitchonEnum_SkillType_Level SkillLevel
    (:NewEnumerator0
      (CallFunction|CallSkill))
    (:NewEnumerator1
      (CallFunction|CallSkill 1))
    (:NewEnumerator2
      (CallFunction|CallSkill 2))))

(event Custom|CallSkill
  (params (Index :type Integer))
  ;[1 0.02399 0] Combat
  ;;[0 1 0.1595] SkillStuff
  (CallFunction|InstantiateSkill (Utilities|Array|Get(acopy) (Variables|Default|GetSkills) Index) (Transformation|GetWorldTransform (Variables|Default|GetRangedSkillPosition))))

(event EventTick
  (params (DeltaSeconds :type Float%20%28single-precision%29))
  ;[1 0.02399 0] Combat
  (CallFunction|CharacterDeathCondition))

(event EventBeginPlay
  ;[0 1 0.1079] Setup
  (CallFunction|SetBasicAttributes (Variables|BasicAttribute|GetPHealth) (Variables|BasicAttribute|GetPMana) (Variables|BasicAttribute|GetPStamina))
  (CallFunction|SetCombatAttributes (Variables|CombatAttributes|GetPDamagePoints)))

(event Input|ActionEvents|InputActionMeeleAttack
  (params (Key :type Key%20Structure :default "None"))
  ;[1 0.02399 0] Combat
  (:Pressed
    (CallFunction|PlayerAttack)))

(event Input|ActionEvents|InputActionBasicSkillAttack
  (params (Key :type Key%20Structure :default "None"))
  ;[1 0.02399 0] Combat
  (:Pressed
    (CallFunction|PlayerExecuteSkill "NewEnumerator0")))

(event Input|AxisEvents|InputAxisMoveForward
  (params (AxisValue :type Float%20%28single-precision%29))
  ;[0 1 0.9729] Movementation & Rotation
  ;;[0 0.9462 1] Movement
  (Pawn|Input|AddMovementInput (Math|Vector|GetForwardVector (Math|Rotator|MakeRotator 0.0 0.0 (.yaw (Pawn|GetControlRotation :!class /Script/Engine.Pawn)))) (* AxisValue (Variables|MovementAttributes|GetMovementSpeed)) false))

(event Input|AxisEvents|InputAxisMoveRight
  (params (AxisValue :type Float%20%28single-precision%29))
  ;[0 1 0.9729] Movementation & Rotation
  ;;[0 0.8141 1] Rotation
  ;;;[1 1 1] Set Rotation
  (Pawn|Input|AddControllerYawInput (* AxisValue (Variables|MovementAttributes|GetRotationSpeed))))

(fn ConstructionScript
  (|CallParentFunction))

(fn InstantiateActor
  (params (Actor :type Actor%20Object%20Reference) (InstanceTransform :type Transform))
  (bind _returnvalue (Game|SpawnActorfromClass (Utilities|GetClass Actor) InstanceTransform "Undefined" 0 0))
  (return _returnvalue))

(fn InstantiateSkill
  (params (SkillClass :type BP%20Skill%20Class%20Reference) (InstatiateTranform :type Transform))
  (bind _actorinstance (CallFunction|InstantiateClass SkillClass InstatiateTranform))
  (bind _asbp_skill (Utilities|Casting|CastToBP_Skill _actorinstance))
  (return _asbp_skill))

(fn InstantiateClass
  (params (Class :type Actor%20Class%20Reference) (InstanceTransform :type Transform))
  (bind _returnvalue (Game|SpawnActorfromClass Class InstanceTransform "Undefined" 0 0))
  (return _returnvalue))